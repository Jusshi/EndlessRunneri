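; Hugo is a 2D flipbook player character that can jump and crouch, with game-only input set on BeginPlay.
; Jump and crouch inputs swap the sprite flipbook, and crouch also shifts the sprite's vertical offset.
; Releasing crouch restores the walk flipbook and offset without calling UnCrouch, and capsule hits on Surface-tagged actors also restore walking.
; The ExitToMenu input opens the MainMenu level.
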(event `self.ReceiveBeginPlay`
  (`WidgetBlueprintLibrary.SetInputMode_GameOnly` (`GameplayStatics.GetPlayerController` 0)))

(event `InputAction|Jump`
  (params (Key :type "Key Structure"))
  (:`Pressed`
    (`PaperFlipbookComponent.SetFlipbook` (`self.Sprite`) "/Game/Flipbookss/Hugo_hyppy.Hugo_hyppy")
    (`self.Jump`)))

(event `InputAction|Crouch`
  (params (Key :type "Key Structure"))
  (:`Pressed`
    (`PaperFlipbookComponent.SetFlipbook` (`self.Sprite`) "/Game/Flipbookss/Hugo_kyyrii.Hugo_kyyrii")
    (`self.Crouch`)
    (`SceneComponent.K2_SetRelativeLocation` (`self.Sprite`) (0.0 0.0 -20.0) false false))
  (:`Released`
    (`PaperFlipbookComponent.SetFlipbook` (`self.Sprite`) "/Game/Flipbookss/Hugonkävely.Hugonkävely")
    (`SceneComponent.K2_SetRelativeLocation` (`self.Sprite`) (0.0 0.0 -10.0) false false)))

(event `self.CapsuleComponent.OnComponentHit`
  (params (HitComponent :type "PrimitiveComponent Object Reference") (OtherActor :type "Actor Object Reference") (OtherComp :type "PrimitiveComponent Object Reference") (NormalImpulse :type "Vector Structure") (Hit :type "HitResult Structure (by ref)"))
  (if (`self.ActorHasTag` OtherActor "Surface")
    (`PaperFlipbookComponent.SetFlipbook` (`self.Sprite`) "/Game/Flipbookss/Hugonkävely.Hugonkävely")))

(event `InputAction|ExitToMenu`
  (params (Key :type "Key Structure"))
  (:`Pressed`
    (`GameplayStatics.OpenLevel` "MainMenu")))

(fn `UserConstructionScript`)