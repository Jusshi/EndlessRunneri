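; Rock actor that spins and signals when its effect is applied.
; Every tick it adds a random pitch rotation in world space, re-rolled each frame and not scaled by delta time, so the spin is uneven and frame-rate dependent.
; ApplyEffect only fires the RockHitED event dispatcher, leaving the response to a hit to whatever is bound to it.
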(event `self.ReceiveTick`
  (params (DeltaSeconds :type "Float (single-precision)"))
  (`parent.ReceiveTick` DeltaSeconds)
  ;[1 1 1] Make the rock rotate in random speed.
  (`self.K2_AddActorWorldRotation` (`KismetMathLibrary.MakeRotator` 0.0 (`KismetMathLibrary.RandomFloatInRange` 1.0 20.0))))

(fn `ApplyEffect`
  (`self.RockHit_ED`))

(fn `UserConstructionScript`
  (`parent.UserConstructionScript`))